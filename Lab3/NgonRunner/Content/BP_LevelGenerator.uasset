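; Level generator that lays out a row of BP_Polygon child actors as an endless course and manages which polygon is selected for rotation.
; Tick detects the player reaching the next polygon, advances the selection and appends polygons once past the first few.
; Every thirty polygons, side count rises up to a maximum and the row steps upward.
; Selection stays within a range ahead of the player, which can be boosted.
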(event `self.ReceiveBeginPlay`
  (bind _returnvalue (`GameplayStatics.GetActorOfClass` "/Game/ThirdPerson/Blueprints/BP_ThirdPersonCharacter.BP_ThirdPersonCharacter_C"))
  (set `self.PlayerReference` _returnvalue)
  (for _ (range (`self.NumOfPolygons`))
    (`self.AddPolygon`)
    (set `self.NumOfPolygons` (- (`self.NumOfPolygons`) 1)))
  (bind _output_get (set `self.SelectedPolygonIndex` 0))
  (bind _aschild_actor_component (cast `ChildActorComponent` (`SceneComponent.GetChildComponent` (`self.DefaultSceneRoot`) _output_get)))
  (bind _asbp_polygon (cast `/Game/BP_Polygon` (`ChildActorComponent.ChildActor` _aschild_actor_component)))
  (`/Game/BP_Polygon.Select` _asbp_polygon))

(event `self.ReceiveTick`
  (params (DeltaSeconds :type "Float (single-precision)"))
  (bind _returnvalue (+ (`self.PlayerPolygonIndex`) 1))
  (bind _returnvalue_2 (> (`self.PlayerPolygonIndex`) 3))
  (bind _returnvalue_3 (== (mod (`self.NumOfPolygons`) 30) 0))
  (bind _aschild_actor_component (cast `ChildActorComponent` (`SceneComponent.GetChildComponent` (`self.DefaultSceneRoot`) _returnvalue)))
  (bind _asbp_polygon (cast `/Game/BP_Polygon` (`ChildActorComponent.ChildActor` _aschild_actor_component)))
  (bind _isplayerhere (`/Game/BP_Polygon.IsPlayerPresent` _asbp_polygon))
  (if _isplayerhere
    (`KismetSystemLibrary.PrintString` "PLAYER AT POLYGON")
    (bind _output_get (set `self.PlayerPolygonIndex` _returnvalue))
    (if (>= _output_get (`self.SelectedPolygonIndex`))
      (`self.SelectNext`))
    (if _returnvalue_2
      (`self.AddPolygon`))
    (if (and (< (`self.PlayerSelectionRange`) 5) (and (not _returnvalue_2) _returnvalue_3))
      (`self.BoostPlayerRange`))
    (if (and _returnvalue_3 (< (`self.CurrentNumOfPolySides`) (`self.MaxNumOfPolySides`)))
      (set `self.CurrentNumOfPolySides` (+ (`self.CurrentNumOfPolySides`) 1))
      (set `self.PolygonPositionTransform` (`KismetMathLibrary.MakeTransform` (+ (.location (`self.PolygonPositionTransform`)) (`KismetMathLibrary.MakeVector` 0.0 0.0 150.0)) (.rotation (`self.PolygonPositionTransform`)) (.scale (`self.PolygonPositionTransform`)))))))

(fn `AddPolygon`
  (bind _polygonpositiontransform (`self.PolygonPositionTransform`))
  (bind _returnvalue (`AddComponent|NODE_AddChildActorComponent-6` :`RelativeTransform` _polygonpositiontransform))
  (`ChildActorComponent.SetChildActorClass` _returnvalue "/Game/BP_Polygon.BP_Polygon_C")
  (bind _asbp_polygon (cast `/Game/BP_Polygon` (`ChildActorComponent.ChildActor` _returnvalue)))
  (set `/Game/BP_Polygon.NumOfSides` (`self.CurrentNumOfPolySides`) _asbp_polygon)
  (`/Game/BP_Polygon.Construct` _asbp_polygon)
  (set `self.PolygonPositionTransform` (`KismetMathLibrary.MakeTransform` (+ (.location _polygonpositiontransform) (`KismetMathLibrary.MakeVector` 0.0 (`self.DistanceBetweenPolygons`)))))
  (set `self.NumOfPolygons` (+ (`self.NumOfPolygons`) 1)))

(fn `BoostPlayerRange`
  (set `self.PlayerSelectionRange` (+ (`self.PlayerSelectionRange`) 1)))

(fn `RotateSelectedLeft`
  (bind _aschild_actor_component (cast `ChildActorComponent` (`SceneComponent.GetChildComponent` (`self.DefaultSceneRoot`) (`self.SelectedPolygonIndex`))))
  (bind _asbp_polygon (cast `/Game/BP_Polygon` (`ChildActorComponent.ChildActor` _aschild_actor_component)))
  (`/Game/BP_Polygon.RotateRight` _asbp_polygon))

(fn `RotateSelectedRight`
  (bind _aschild_actor_component (cast `ChildActorComponent` (`SceneComponent.GetChildComponent` (`self.DefaultSceneRoot`) (`self.SelectedPolygonIndex`))))
  (bind _asbp_polygon (cast `/Game/BP_Polygon` (`ChildActorComponent.ChildActor` _aschild_actor_component)))
  (`/Game/BP_Polygon.RotateLeft` _asbp_polygon))

(fn `SelectNext`
  (bind _selectedpolygonindex (`self.SelectedPolygonIndex`))
  (if (and (< _selectedpolygonindex (+ (`self.PlayerPolygonIndex`) (`self.PlayerSelectionRange`))) (< _selectedpolygonindex (- (`self.NumOfPolygons`) 1)))
    (bind _aschild_actor_component (cast `ChildActorComponent` (`SceneComponent.GetChildComponent` (`self.DefaultSceneRoot`) (`self.SelectedPolygonIndex`))))
    (bind _asbp_polygon (cast `/Game/BP_Polygon` (`ChildActorComponent.ChildActor` _aschild_actor_component)))
    (`/Game/BP_Polygon.Unselect` _asbp_polygon)
    (bind _output_get (set `self.SelectedPolygonIndex` (+ _selectedpolygonindex 1)))
    (bind _aschild_actor_component_2 (cast `ChildActorComponent` (`SceneComponent.GetChildComponent` (`self.DefaultSceneRoot`) _output_get)))
    (bind _asbp_polygon_2 (cast `/Game/BP_Polygon` (`ChildActorComponent.ChildActor` _aschild_actor_component_2)))
    (`/Game/BP_Polygon.Select` _asbp_polygon_2)
    (else
      (`KismetSystemLibrary.PrintString` (`KismetStringLibrary.Conv_IntToString` (`self.PlayerPolygonIndex`)))
      (`KismetSystemLibrary.PrintString` (`KismetStringLibrary.Conv_IntToString` (`self.SelectedPolygonIndex`))))))

(fn `SelectPrevious`
  (bind _selectedpolygonindex (`self.SelectedPolygonIndex`))
  (if (> _selectedpolygonindex (+ (`self.PlayerPolygonIndex`) 1))
    (bind _aschild_actor_component (cast `ChildActorComponent` (`SceneComponent.GetChildComponent` (`self.DefaultSceneRoot`) (`self.SelectedPolygonIndex`))))
    (bind _asbp_polygon (cast `/Game/BP_Polygon` (`ChildActorComponent.ChildActor` _aschild_actor_component)))
    (`/Game/BP_Polygon.Unselect` _asbp_polygon)
    (bind _output_get (set `self.SelectedPolygonIndex` (- _selectedpolygonindex 1)))
    (bind _aschild_actor_component_2 (cast `ChildActorComponent` (`SceneComponent.GetChildComponent` (`self.DefaultSceneRoot`) _output_get)))
    (bind _asbp_polygon_2 (cast `/Game/BP_Polygon` (`ChildActorComponent.ChildActor` _aschild_actor_component_2)))
    (`/Game/BP_Polygon.Select` _asbp_polygon_2)
    (else
      (`KismetSystemLibrary.PrintString` "Hello"))))

(fn `UserConstructionScript`
  (set `self.PlayerPolygonIndex` -1)
  (set `self.CurrentNumOfPolySides` (`self.MinNumOfPolySides`)))