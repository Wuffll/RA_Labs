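; Rotatable polygon platform that tracks whether the player is inside its presence box and updates the HUD score on entry.
; Construct, not the construction script, builds a ring of randomly picked tile child actors from the side count and length.
; RotateRight and RotateLeft queue one-side pitch steps, which Tick plays as an eased timeline, refusing overlapping turns.
; Select and Unselect toggle custom depth on the tile meshes for highlighting.
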(event `self.ReceiveTick`
  (params (DeltaSeconds :type "Float (single-precision)"))
  (if (`self.IsRotating`)
    _
    (elif (`self.RotationNeeded`)
      (set `self.IsRotating` true)
      (`TimelineComponent.SetTimelineLength` (`self.Lerp Timeline`) (`self.RotationTimeLength`))
      (`Timeline|Lerp Timeline` :!via `PlayFromStart`
        (:`Update`
          (`SceneComponent.K2_SetRelativeRotation` (`self.DefaultSceneRoot`) (`|EaseFunction` (`self.RotationEasingFunction`) (`KismetMathLibrary.FClamp` (/ (`TimelineComponent.GetPlaybackPosition` (`self.Lerp Timeline`)) (`self.RotationTimeLength`))) (`self.StartRot`) (`self.EndRot`)) false false))
        (:`Finished`
          (set `self.IsRotating` false)
          (set `self.RotationNeeded` false))))))

(event `self.PresenceBox.OnComponentBeginOverlap`
  (params (OverlappedComponent :type "PrimitiveComponent Object Reference") (OtherActor :type "Actor Object Reference") (OtherComp :type "PrimitiveComponent Object Reference") (OtherBodyIndex :type Integer) (bFromSweep :type Boolean) (SweepResult :type "HitResult Structure (by ref)"))
  (cast `/Game/ThirdPerson/Blueprints/BP_ThirdPersonCharacter` OtherActor)
  (set `self.IsPlayerHere` true)
  (`KismetSystemLibrary.PrintString` "Entered")
  (bind _asscore_hud (cast `/Game/Blueprints/ScoreHUD` (`PlayerController.GetHUD` (`GameplayStatics.GetPlayerController` 0))))
  (`/Game/BP_ScoreHUDWidget.UpdateScore` (`/Game/Blueprints/ScoreHUD.UIReference` _asscore_hud)))

(event `self.PresenceBox.OnComponentEndOverlap`
  (params (OverlappedComponent :type "PrimitiveComponent Object Reference") (OtherActor :type "Actor Object Reference") (OtherComp :type "PrimitiveComponent Object Reference") (OtherBodyIndex :type Integer))
  (cast `/Game/ThirdPerson/Blueprints/BP_ThirdPersonCharacter` OtherActor)
  (set `self.IsPlayerHere` false))

(fn `Construct`
  (locals (DistMiddleToSideCenter :type "Float (double-precision)") (NewSidePosition :type "Vector Structure") (Angle :type "Float (double-precision)"))
  (bind _tiletypesarray (`self.TileTypesArray`))
  (if (!= (`KismetArrayLibrary.Array_Length` _tiletypesarray) 0)
    (bind _output_get (set `local.Angle` (/ 360.0 (`KismetMathLibrary.Conv_IntToDouble` (`self.NumOfSides`)))))
    (bind _output_get_2 (set `local.DistMiddleToSideCenter` (/ (* (`self.SideLength`) 100.0) (`KismetMathLibrary.DegTan` (/ _output_get 2.0)))))
    (set `local.NewSidePosition` (`KismetMathLibrary.MakeVector` 0.0 0.0 (* _output_get_2 -1.0)))
    (for _index (range (+ (+ (`self.NumOfSides`) -1) 1))
      (bind _returnvalue (`AddComponent|NODE_AddChildActorComponent-4` :`RelativeTransform` (`KismetMathLibrary.MakeTransform` (`local.NewSidePosition`) (`KismetMathLibrary.MakeRotator` 0.0 (* (* _index -1) (`local.Angle`))))))
      (`ChildActorComponent.SetChildActorClass` _returnvalue (`KismetArrayLibrary.Array_Random` _tiletypesarray))
      (cast `/Game/BP_Tile_Active` (`ChildActorComponent.ChildActor` _returnvalue)
        (:`then`
          (set `local.NewSidePosition` (`KismetMathLibrary.RotateAngleAxis` (`local.NewSidePosition`) (`local.Angle`) (0.0 1.0 0.0))))
        (:`CastFailed`
          (`KismetSystemLibrary.PrintString` "ERROR: Can't cast to BP_Tile_Active"))))
    (set `self.TileTypesArray` (`|MakeArray` null :!type "Actor Class Reference"))))

(fn `IsPlayerPresent`
  (returns (IsPlayerHere :type Boolean))
  (return (`self.IsPlayerHere`)))

(fn `RotateLeft`
  (locals (StartRotation :type "Rotator Structure") (EndRotation :type "Rotator Structure"))
  (bind _endrot (`self.EndRot`))
  (if (`self.RotationNeeded`)
    (`KismetSystemLibrary.PrintString` "Already rotating!")
    (else
      (set `self.RotationNeeded` true)
      (set `self.StartRot` _endrot)
      (bind _output_get (set `self.EndRot` (`KismetMathLibrary.MakeRotator` (.roll _endrot) (`KismetMathLibrary.NormalizeAxis` (+ (`KismetMathLibrary.ClampAxis` (.pitch _endrot)) (* (/ -360.0 (`KismetMathLibrary.Conv_IntToDouble` (`self.NumOfSides`))) 1.0))) (.yaw _endrot))))
      (`KismetSystemLibrary.PrintString` (`KismetStringLibrary.Conv_RotatorToString` _output_get) true true (struct :`G` 0.66 :`B` 1.0 :`A` 1.0) 1000.0)
      (`KismetSystemLibrary.PrintString` (`KismetStringLibrary.Conv_RotatorToString` (`self.StartRot`)) true true (struct :`G` 0.66 :`B` 1.0 :`A` 1.0) 1000.0))))

(fn `RotateRight`
  (bind _endrot (`self.EndRot`))
  (if (`self.RotationNeeded`)
    (`KismetSystemLibrary.PrintString` "Already rotating!")
    (else
      (set `self.RotationNeeded` true)
      (set `self.StartRot` _endrot)
      (bind _output_get (set `self.EndRot` (`KismetMathLibrary.MakeRotator` (.roll _endrot) (`KismetMathLibrary.NormalizeAxis` (+ (`KismetMathLibrary.ClampAxis` (.pitch _endrot)) (* (/ 360.0 (`KismetMathLibrary.Conv_IntToDouble` (`self.NumOfSides`))) 1.0))) (.yaw _endrot))))
      (`KismetSystemLibrary.PrintString` (`KismetStringLibrary.Conv_RotatorToString` _output_get) true true (struct :`G` 0.66 :`B` 1.0 :`A` 1.0) 1000.0)
      (`KismetSystemLibrary.PrintString` (`KismetStringLibrary.Conv_RotatorToString` (`self.StartRot`)) true true (struct :`G` 0.66 :`B` 1.0 :`A` 1.0) 1000.0))))

(fn `Select`
  (for _array_element (`SceneComponent.GetChildrenComponents` (`self.DefaultSceneRoot`) false)
    (bind _aschild_actor_component (cast `ChildActorComponent` _array_element))
    (bind _asbp_tile_active (cast `/Game/BP_Tile_Active` (`ChildActorComponent.ChildActor` _aschild_actor_component)))
    (`PrimitiveComponent.SetRenderCustomDepth` (`/Game/BP_Tile.StaticMesh` _asbp_tile_active) true)))

(fn `Unselect`
  (for _array_element (`SceneComponent.GetChildrenComponents` (`self.DefaultSceneRoot`) false)
    (bind _aschild_actor_component (cast `ChildActorComponent` _array_element))
    (bind _asbp_tile_active (cast `/Game/BP_Tile_Active` (`ChildActorComponent.ChildActor` _aschild_actor_component)))
    (`PrimitiveComponent.SetRenderCustomDepth` (`/Game/BP_Tile.StaticMesh` _asbp_tile_active) false)))

(fn `UserConstructionScript`
  ;[1 1 1] USE FUNCTION CONSTRUCT !!!
)