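; Level generator that builds a row of rotatable BP_Polygon segments and tracks the player's progress along it.
; The construction script spawns the segments as child actor components evenly spaced along Y.
; Tick polls the segment before the player's index, counting down as the player arrives and keeping the selection below that index.
; Functions move the selection within PlayerSelectionRange and rotate the selected polygon left or right.
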(event `self.ReceiveBeginPlay`)

(event `self.ReceiveTick`
  (params (DeltaSeconds :type "Float (single-precision)"))
  (bind _selectedpolygonindex (`self.SelectedPolygonIndex`))
  (bind _returnvalue (+ (`self.PlayerPolygonIndex`) -1))
  (bind _aschild_actor_component (cast `ChildActorComponent` (`SceneComponent.GetChildComponent` (`self.DefaultSceneRoot`) _returnvalue)))
  (bind _asbp_polygon (cast `/Game/BP_Polygon` (`ChildActorComponent.ChildActor` _aschild_actor_component)))
  (bind _isplayerhere (`/Game/BP_Polygon.IsPlayerPresent` _asbp_polygon))
  (if _isplayerhere
    (`KismetSystemLibrary.PrintString` "PLAYER AT POLYGON")
    (bind _output_get (set `self.PlayerPolygonIndex` _returnvalue))
    (if (<= _output_get _selectedpolygonindex)
      (set `self.SelectedPolygonIndex` (- _selectedpolygonindex (+ (- _selectedpolygonindex (`self.PlayerPolygonIndex`)) 1))))))

(fn `RotateSelectedLeft`
  (bind _aschild_actor_component (cast `ChildActorComponent` (`SceneComponent.GetChildComponent` (`self.DefaultSceneRoot`) (`self.SelectedPolygonIndex`))))
  (bind _asbp_polygon (cast `/Game/BP_Polygon` (`ChildActorComponent.ChildActor` _aschild_actor_component)))
  (`/Game/BP_Polygon.RotateLeft` _asbp_polygon))

(fn `RotateSelectedRight`
  (bind _aschild_actor_component (cast `ChildActorComponent` (`SceneComponent.GetChildComponent` (`self.DefaultSceneRoot`) (`self.SelectedPolygonIndex`))))
  (bind _asbp_polygon (cast `/Game/BP_Polygon` (`ChildActorComponent.ChildActor` _aschild_actor_component)))
  (`/Game/BP_Polygon.Rotate Right` _asbp_polygon))

(fn `SelectNext`
  (bind _playerpolygonindex (`self.PlayerPolygonIndex`))
  (bind _selectedpolygonindex (`self.SelectedPolygonIndex`))
  (bind _returnvalue (- _playerpolygonindex (`KismetMathLibrary.Min` _playerpolygonindex (`self.PlayerSelectionRange`))))
  (if (and (> _selectedpolygonindex _returnvalue) (>= _returnvalue 0))
    (set `self.SelectedPolygonIndex` (- _selectedpolygonindex 1))
    (else
      (`KismetSystemLibrary.PrintString` "Hello"))))

(fn `SelectPrevious`
  (bind _selectedpolygonindex (`self.SelectedPolygonIndex`))
  (if (< _selectedpolygonindex (- (`self.PlayerPolygonIndex`) 1))
    (set `self.SelectedPolygonIndex` (+ _selectedpolygonindex 1))))

(fn `UserConstructionScript`
  (bind _numofpolygons (`self.NumOfPolygons`))
  (set `self.PlayerPolygonIndex` _numofpolygons)
  (bind _output_get (set `self.SelectedPolygonIndex` (- _numofpolygons 1)))
  (for _index (range (+ _output_get 1))
    (bind _returnvalue (`AddComponent|NODE_AddChildActorComponent-0` :`RelativeTransform` (`KismetMathLibrary.MakeTransform` (+ (.location (`self.StartingTransform`)) (`KismetMathLibrary.MakeVector` 0.0 (* (`KismetMathLibrary.Conv_IntToDouble` _index) 830.0))))))
    (`ChildActorComponent.SetChildActorClass` _returnvalue "/Game/BP_Polygon.BP_Polygon_C")))